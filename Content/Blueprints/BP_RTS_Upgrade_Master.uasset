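; Base class for RTS upgrades, defining the shared interface for unlocking, affordability checks and activation.
; ShouldBeUnlocked passes when the RequiredUpgrades list is empty or every entry appears in the supplied bought-upgrade list.
; Activate forwards the controller to DepleteResources, an empty event here.
; HasEnoughResources is a stub that each upgrade is meant to implement with its own resource check.
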(event Custom|Activate
  (params (Instigator :type Actor%20Object%20Reference) (Controller :type BP%20RTS%20Controller%20Object%20Reference))
  (CallFunction|DepleteResources Controller))

(event Custom|DepleteResources
  (params (Owner :type BP%20RTS%20Controller%20Object%20Reference)))

(event EventBeginPlay)

(fn ConstructionScript)

(fn ShouldbeUnlocked
  (params (BoughtUpgradeList :type Array%20of%20BP%20RTS%20Upgrade%20Master%20Class%20References))
  (Utilities|FlowControl|Sequence
    (:then_0
      (if (== (Utilities|Array|Length (Variables|Default|GetRequiredUpgrades)) 0)
        (LocalVariables|SetbShouldBeUnlocked true)
        (else
          (for _array_element (Variables|Default|GetRequiredUpgrades)
            (if (Utilities|Array|ContainsItem BoughtUpgradeList _array_element)
              (LocalVariables|SetNumValidUpgrades (+ (LocalVariables|GetNumValidUpgrades) 1))))
          (if (>= (LocalVariables|GetNumValidUpgrades) (Utilities|Array|Length (Variables|Default|GetRequiredUpgrades)))
            (LocalVariables|SetbShouldBeUnlocked true)))))
    (:then_1
      (return (LocalVariables|GetbShouldBeUnlocked)))))

(fn HasEnoughResources
  (params (Controller :type BP%20RTS%20Controller%20Object%20Reference))
  ;[1 1 1] Implement this in each upgrade
  (return (LocalVariables|GetbHasEnough)))