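; BP_ConstructionProxy is a base Blueprint for an in-progress construction job that tracks work hours until completion.
; Each Tick adds assigned worker count times scaled delta time, using TimeScale from a cached BP_RTS_GameState, capped at the hours needed.
; Completion sets a flag and calls CallConstructionCompleted.
; Derived Blueprints override empty post-create and post-work hooks, while Initialize's RateMultiplier input is unused.
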(event `self.ReceiveTick`
  (params (DeltaSeconds :type "Float (single-precision)"))
  (if (not (`self.ConstructionComplete`))
    (`self.DoWork` DeltaSeconds)
    (`self.DoPostWorkUpdate`)
    (if (>= (`self.WorkHoursSpent`) (`self.WorkHoursNeeded`))
      (set `self.ConstructionComplete` true)
      (`self.ConstructionCompleted` self))))

(fn `DoPostInitUpdate`
  ;[1 1 1] NOT USED at the moment
)

(fn `DoPostWorkUpdate`
  ;[1 1 1] This function will do whatever update is needed after doing work. Should be overiden in derived BPs
)

(fn `DoWork`
  (params (DeltaSeconds :type "Float (double-precision)"))
  (bind _gamestate (`self.GetCachedGameStateRef`)
    (:`Valid`
      (set `self.WorkHoursSpent` (`KismetMathLibrary.FMin` (+ (/ (* (`self.GetEffectiveWorkForce`) (* (`/Game/Blueprints/BP_RTS_GameState.TimeScale` _gamestate) DeltaSeconds)) 3600.0) (`self.WorkHoursSpent`)) (`self.WorkHoursNeeded`))))))

(fn `GetEffectiveWorkForce`
  (returns (WorkForce :type "Float (double-precision)"))
  (return (`KismetMathLibrary.Conv_IntToDouble` (`KismetArrayLibrary.Array_Length` (`self.AssignedWorkers`)))))

(fn `Initialize`
  (params (WorkHoursNeeded :type "Float (double-precision)") (RateMultiplier :type "Float (double-precision)"))
  (set `self.WorkHoursNeeded` WorkHoursNeeded)
  (`self.OnPostCreate`))

(fn `OnPostCreate`
  ;[1 1 1] Do anything you want after initialization. Override in derived BPs
)

(fn `SetWorkers`
  (params (Workers :type "Array of Integer"))
  (set `self.AssignedWorkers` Workers))

(fn `UserConstructionScript`)