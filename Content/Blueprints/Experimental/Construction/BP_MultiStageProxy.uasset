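; Experimental multi-stage construction proxy that changes its appearance and effects as work hours accumulate.
; It activates the first stage on creation, then after each work update advances at most one stage once completion percentage exceeds the active stage's threshold.
; Each stage swaps in its mesh, sound and particle system, switching off audio or particles it lacks but keeping the previous mesh if none is set.
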(event `self.DoPostWorkUpdate`
  (bind _stage (`self.GetActiveStage`)
    (:`Valid`
      (if (> (* 100 (/ (`self.WorkHoursSpent`) (`self.WorkHoursNeeded`))) (`.Percentage_23_8ED36AEE459753E57B3F339D340BEB4E` (break `/Game/Blueprints/Experimental/Construction/STRUCT_ConstructionStage` _stage)))
        (`self.AdvanceStage`)))))

(event `self.OnPostCreate`
  (`self.ActivateStage` (`KismetArrayLibrary.Array_Get` (`self.Stages`))))

(fn `ActivateStage`
  (params (Stage :type "/Game/Blueprints/Experimental/Construction/STRUCT_ConstructionStage Structure"))
  (bind (_percentage _mesh _sound _particlesystem) (break `/Game/Blueprints/Experimental/Construction/STRUCT_ConstructionStage` Stage))
  (bind _audio (`self.Audio`))
  (bind _particlesystem_2 (`self.ParticleSystem`))
  (`|ExecutionSequence`
    (:`then_0`
      (`/Engine/EditorBlueprintResources/StandardMacros.IsValid` _mesh
        (:`Is Valid`
          (`StaticMeshComponent.SetStaticMesh` (`self.Mesh`) _mesh))))
    (:`then_1`
      (`/Engine/EditorBlueprintResources/StandardMacros.IsValid` _sound
        (:`Is Valid`
          (`AudioComponent.SetSound` _audio _sound)
          (`ActorComponent.Activate` _audio false))
        (:`Is Not Valid`
          (`ActorComponent.Deactivate` _audio))))
    (:`then_2`
      (`/Engine/EditorBlueprintResources/StandardMacros.IsValid` _particlesystem
        (:`Is Valid`
          (`ParticleSystemComponent.SetTemplate` _particlesystem_2 _particlesystem)
          (`ActorComponent.Activate` _particlesystem_2 false))
        (:`Is Not Valid`
          (`ActorComponent.Deactivate` _particlesystem_2))))))

(fn `AdvanceStage`
  (bind _currentstageindex (`self.CurrentStageIndex`))
  (bind _stages (`self.Stages`))
  (bind _returnvalue (+ _currentstageindex 1))
  (if (and (>= _returnvalue 0) (< _returnvalue (`KismetArrayLibrary.Array_Length` _stages)))
    (set `self.CurrentStageIndex` _returnvalue)
    (`self.ActivateStage` (`KismetArrayLibrary.Array_Get` _stages _currentstageindex))))

(fn `UserConstructionScript`
  (`parent.UserConstructionScript`))