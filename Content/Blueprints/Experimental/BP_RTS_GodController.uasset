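; Experimental RTS god-style controller that lets the player place barracks with the mouse.
; On BeginPlay it spawns a construction manager and keeps a reference to it.
; Each left-click, gated by a DoOnce that resets on release, queues a barrack and its proxy at the cursor trace hit, aligned to the surface normal.
; Building class and work time are hard-coded.
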(event `self.ReceiveBeginPlay`
  (bind _returnvalue (`|SpawnActorFromClass` "/Game/Blueprints/Experimental/Construction/BP_ConstructionManager.BP_ConstructionManager_C" (`KismetMathLibrary.MakeTransform` (0.0 0.0 0.0))))
  (set `self.ConstructionManager` _returnvalue))

(event `InputAction|LMB`
  (bind (_location _normal) (`GameplayStatics.BreakHitResult` (`self.GetHitResultUnderCursorByChannel` "TraceTypeQuery3")))
  (:`Pressed`
    (`/Engine/EditorBlueprintResources/StandardMacros.DoOnce` false :!label _label
      (:`Completed`
        (`/Game/Blueprints/Experimental/Construction/BP_ConstructionManager.QueueConstruction` (`self.ConstructionManager`) (make `/Game/Blueprints/Experimental/Construction/STRUCT_ConstructionConf` "/Game/Blueprints/Experimental/Construction/Barrack/BP_Barrack.BP_Barrack_C" "/Game/Blueprints/Experimental/Construction/Barrack/BP_BarrackProxy.BP_BarrackProxy_C" (`KismetMathLibrary.MakeTransform` _location (`KismetMathLibrary.MakeRotFromZ` _normal)) 0.005)))))
  (:`Released`
    (goto _label :!via `Reset`)))

(fn `UserConstructionScript`)