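; Experimental RTS "god" camera that pans, zooms and yaw-rotates while a rotation-mode trigger is held.
; Pan and zoom inputs set a target location, which Tick interpolates toward, with curves scaling speed and optionally spring-arm tilt by zoom.
; Line traces along the camera's view keep it within min/max distance of the surface hit and cache a pivot.
; Rotation only yaws the actor in place, as the pivot-orbit node is unconnected.
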(event EventTick
  (params (DeltaSeconds :type Float%20%28single-precision%29))
  (bind _returnvalue (Transformation|GetActorLocation))
  (bind _targetgodlocation (Variables|Default|GetTargetGodLocation))
  (bind _targetgodlocation_2 (Variables|Default|GetTargetGodLocation))
  (bind _springarm (Variables|Default|GetSpringArm))
  (bind _returnvalue_2 (- _returnvalue _targetgodlocation_2))
  (bind _relativerotation (Variables|/Script/Engine.SceneComponent|GetRelativeRotation _springarm))
  (bind _returnvalue_3 (Math|Vector|VectorLength _returnvalue_2))
  (bind (_pitch _yaw _roll) (Class|KismetMathLibrary|BreakRot _relativerotation))
  (bind _returnvalue_4 (Math|Float|Absolute(Float) _returnvalue_3))
  ;[1 1 1] Tick and Interpolation
  (if (not (Variables|Default|GetbInRotationMode))
    (if (> _returnvalue_4 (Variables|Default|GetInterpTolerance))
      (Transformation|SetActorLocation (Math|Interpolation|VInterpTo (Transformation|GetActorLocation) _targetgodlocation DeltaSeconds 1e+01) false)
      (CallFunction|UpdatePivotCache :!label _label)
      (Variables|Default|SetApproximateCameraDistance (Math|Float|Absolute(Float) (Math|Vector|VectorLength (- (Transformation|GetActorLocation) (Variables|Default|GetCachedRotationPivot)))))
      (if (Variables|Default|GetAutoTiltBasedOnZoom)
        (Transformation|SetRelativeRotation _springarm (Class|KismetMathLibrary|MakeRot (Math|Curves|GetFloatValue (Variables|Default|GetTiltVsDistanceCurve) (Utilities|GetDistanceRatio)) _yaw _roll) false))
      (elif (> _returnvalue_4 0.001)
        (Transformation|SetActorLocation _targetgodlocation false)
        (goto _label)))))

(event EventBeginPlay
  (bind _initialcameradistance (Variables|Default|GetInitialCameraDistance))
  ;[1 1 1] Initialization
  (Transformation|SetRelativeRotation (Variables|Default|GetSpringArm) (Class|KismetMathLibrary|MakeRot (Variables|Default|GetTiltAngle) 0.0 0.0) false)
  (Variables|Default|SetTargetTiltAngle 0.0)
  (Variables|Default|SetDesiredCameraDistance _initialcameradistance)
  (Variables|Default|SetApproximateCameraDistance _initialcameradistance)
  (CallFunction|MoveCameratoDistance _initialcameradistance false 0.0 false))

(event Input|ActionEvents|InputActionCameraZoomIn
  ;[1 1 1] Zooming
  (:Pressed
    (Utilities|MergeZoomInputs (stale Input|AxisEvents|InputAxisZoom AxisValue)) ; enters at ZoomInPressed
  ))

(event Input|ActionEvents|InputActionCameraZoomOut
  ;[1 1 1] Zooming
  (:Pressed
    (Utilities|MergeZoomInputs (stale Input|AxisEvents|InputAxisZoom AxisValue)) ; enters at ZoomOutPressed
  ))

(event Input|ActionEvents|InputActionRotationModeTrigger
  ;[1 1 1] Rotation
  (:Pressed
    (Variables|Default|SetbInRotationMode true))
  (:Released
    (Variables|Default|SetbInRotationMode false)
    (Variables|Default|SetbIsCachedPivotValid false)))

(event Input|AxisEvents|InputAxisMoveForward
  (params (AxisValue :type Float%20%28single-precision%29))
  ;[1 1 1] WASD Movement
  (Utilities|HasMovementInput AxisValue (stale Input|AxisEvents|InputAxisMoveRight AxisValue)
    (:Yes
      (if (not (Variables|Default|GetbInRotationMode))
        (bind _next_location (CallFunction|CalculateNextLocationfromInputs AxisValue (stale Input|AxisEvents|InputAxisMoveRight AxisValue)))
        (CallFunction|MoveCameratoLocation _next_location true)))))

(event Input|AxisEvents|InputAxisMoveRight
  (params (AxisValue :type Float%20%28single-precision%29))
  ;[1 1 1] WASD Movement
  (Utilities|HasMovementInput (stale Input|AxisEvents|InputAxisMoveForward AxisValue) AxisValue
    (:Yes
      (if (not (Variables|Default|GetbInRotationMode))
        (bind _next_location (CallFunction|CalculateNextLocationfromInputs (stale Input|AxisEvents|InputAxisMoveForward AxisValue) AxisValue))
        (CallFunction|MoveCameratoLocation _next_location true)))))

(event Input|AxisEvents|InputAxisZoom
  (params (AxisValue :type Float%20%28single-precision%29))
  ;[1 1 1] Zooming
  (bind _effective_zoom (Utilities|MergeZoomInputs AxisValue)
    (:Exec
      (if (not (Variables|Default|GetbInRotationMode))
        (if (> (Math|Float|Absolute(Float) _effective_zoom) 0.0)
          (Variables|Default|SetDesiredCameraDistance (Math|Float|Min(Float) (Math|Float|Max(Float) (+ (* _effective_zoom (Math|Curves|GetFloatValue (Variables|Default|GetSpeedVsDistanceCurve) (Utilities|GetDistanceRatio)) 3e+01) (Variables|Default|GetApproximateCameraDistance)) (Variables|Default|GetMinCameraDistance)) (Variables|Default|GetMaxCameraDistance)))
          (CallFunction|MoveCameratoDistance (Math|Float|Min(Float) (Math|Float|Max(Float) (+ (* _effective_zoom (Math|Curves|GetFloatValue (Variables|Default|GetSpeedVsDistanceCurve) (Utilities|GetDistanceRatio)) 3e+01) (Variables|Default|GetApproximateCameraDistance)) (Variables|Default|GetMinCameraDistance)) (Variables|Default|GetMaxCameraDistance)) true 0.0 true))))))

(event Input|AxisEvents|InputAxisCameraRotation
  (params (AxisValue :type Float%20%28single-precision%29))
  ;[1 1 1] Rotation
  (if (and (not (Variables|Default|GetbInAxisRotation)) (Variables|Default|GetbInRotationMode))
    (CallFunction|ProcessRotationInput AxisValue)
    (else
      (Variables|Default|SetbInRotationMode false)
      (Variables|Default|SetbIsCachedPivotValid false))))

(fn ConstructionScript)

(fn MoveCameratoDistance
  (params (Distance :type Float%20%28single-precision%29) (bInterpolate :type Boolean) (InterpolationRate :type Float%20%28single-precision%29) (bConstraintDistance :type Boolean))
  (Variables|Default|SetDesiredCameraDistance Distance)
  (bind (_safelocation _distance) (CallFunction|CalculateSafeGodLocation (Variables|Default|GetTargetGodLocation) Distance bConstraintDistance))
  (Variables|Default|SetTargetGodLocation _safelocation)
  (if (not bInterpolate)
    (Variables|Default|SetApproximateCameraDistance _distance)
    (Transformation|SetActorLocation _safelocation false)))

(fn CalculateSafeGodLocation
  (params (FocalPoint :type Vector) (CameraDistance :type Float%20%28single-precision%29) (bContraintDistance :type Boolean))
  (bind _camera (Variables|Default|GetCamera))
  (bind _returnvalue (Transformation|GetWorldRotation _camera))
  (bind _returnvalue_2 (Math|Rotator|GetRotationXVector _returnvalue))
  (bind _outhit (Collision|LineTraceByChannel FocalPoint (+ FocalPoint (* _returnvalue_2 (Variables|Default|GetMaxTraceDistance))) "TraceTypeQuery3" false 0 "None"))
  (if bContraintDistance
    (LocalVariables|SetConstrainedDistance (Math|Float|Max(Float) (Math|Float|Min(Float) CameraDistance (Variables|Default|GetMaxCameraDistance)) (Variables|Default|GetMinCameraDistance)))
    (else
      (LocalVariables|SetConstrainedDistance CameraDistance)))
  (return (+ (.Location (Collision|BreakHitResult _outhit)) (* (* _returnvalue_2 -1.0) (LocalVariables|GetConstrainedDistance))) (Math|Vector|VectorLength (* (* _returnvalue_2 -1.0) (LocalVariables|GetConstrainedDistance)))))

(fn MoveCameratoLocation
  (params (Location :type Vector) (bInterpolate :type Boolean))
  (bind _camera (Variables|Default|GetCamera))
  (bind _mincameradistance (Variables|Default|GetMinCameraDistance))
  (bind _maxcameradistance (Variables|Default|GetMaxCameraDistance))
  (bind _returnvalue (Transformation|GetWorldRotation _camera))
  (bind _returnvalue_2 (Math|Rotator|GetRotationXVector _returnvalue))
  (bind _returnvalue_3 (* _returnvalue_2 -1.0))
  (bind (_outhit _returnvalue_4) (Collision|LineTraceByChannel Location (+ Location (* _returnvalue_2 (Variables|Default|GetMaxTraceDistance))) "TraceTypeQuery3" false 0 "None"))
  (if _returnvalue_4
    (if (>= (Math|Float|Absolute(Float) (Math|Vector|VectorLength (- Location (.Location (Collision|BreakHitResult _outhit))))) _mincameradistance)
      (if (<= (Math|Float|Absolute(Float) (Math|Vector|VectorLength (- Location (.Location (Collision|BreakHitResult _outhit))))) _maxcameradistance)
        (LocalVariables|SetSafe%20Location Location)
        (else
          (LocalVariables|SetSafe%20Location (+ (* _returnvalue_3 (- _maxcameradistance 1.0)) (.Location (Collision|BreakHitResult _outhit))))))
      (else
        (LocalVariables|SetSafe%20Location (+ (* _returnvalue_3 (+ _mincameradistance 1.0)) (.Location (Collision|BreakHitResult _outhit))))))
    (Variables|Default|SetTargetGodLocation (LocalVariables|GetSafe%20Location))
    (if (not bInterpolate)
      (Transformation|SetActorLocation (LocalVariables|GetSafe%20Location) false)
      (Variables|Default|SetCachedRotationPivot (.Location (Collision|BreakHitResult _outhit)))
      (Variables|Default|SetbIsCachedPivotValid false))))

(fn CalculateNextLocationfromInputs
  (params (Forward :type Float%20%28single-precision%29) (Right :type Float%20%28single-precision%29))
  (bind (_normalizedforward _normalizedright) (Utilities|NormalizeMoveInput Forward Right))
  (return (+ (* (+ (* (Transformation|GetActorForwardVector) _normalizedforward) (* (Transformation|GetActorRightVector) _normalizedright)) (Math|Curves|GetFloatValue (Variables|Default|GetSpeedVsDistanceCurve) (Utilities|GetDistanceRatio))) (Variables|Default|GetTargetGodLocation))))

(fn ProcessRotationInput
  (params (Input :type Float%20%28single-precision%29))
  (if (Variables|Default|GetbIsCachedPivotValid)
    _
    (else
      (CallFunction|UpdatePivotCache)))
  (CallFunction|RotateCamerabyAngle (Variables|Default|GetCachedRotationPivot) (* Input (Variables|Default|GetRotationRate))))

(fn RotateCamerabyAngle
  (params (Pivot :type Vector) (Angle :type Float%20%28single-precision%29))
  (Transformation|SetActorRotation (Math|Rotator|CombineRotators (Class|KismetMathLibrary|MakeRot 0.0 Angle 0.0) (Transformation|GetActorRotation))))

(fn UpdatePivotCache
  (bind _returnvalue (Transformation|GetActorLocation))
  (bind _outhit (Collision|LineTraceByChannel _returnvalue (+ _returnvalue (* (Math|Rotator|GetRotationXVector (Transformation|GetWorldRotation (Variables|Default|GetCamera))) (Variables|Default|GetMaxTraceDistance))) "TraceTypeQuery3" false 0 "None"))
  (Variables|Default|SetCachedRotationPivot (.Location (Collision|BreakHitResult _outhit)))
  (Variables|Default|SetbIsCachedPivotValid true))