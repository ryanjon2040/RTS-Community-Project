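; RTS game mode that spawns the upgrade manager on BeginPlay, assigns player starts and registers teams.
; PostLogin caches the newest player as CurrentPlayer for use in player start selection.
; A C++ override event returns the first BP_RTS_PlayerStart found through a variable and conditionally notifies that start of the cached player's spawn.
; RegisterTeam adds unseen teams to the Teams array and returns the new index as a byte.
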(event `self.ReceiveBeginPlay`
  (`parent.ReceiveBeginPlay`)
  (bind _returnvalue (`|SpawnActorFromClass` "/Game/Blueprints/Upgrades/BP_RTS_UpgradeManager.BP_RTS_UpgradeManager_C" (`KismetMathLibrary.MakeTransform` (0.0 0.0 0.0)) true))
  (set `self.UpgradeManager` _returnvalue))

(event `self.CPPOverride_FindPlayerStart`
  (bind _outactors (`GameplayStatics.GetAllActorsOfClass` "/Game/Blueprints/BP_RTS_PlayerStart.BP_RTS_PlayerStart_C"))
  (bind _item (`KismetArrayLibrary.Array_Get` _outactors))
  (set `self.CPPOverrideVar_FindPlayerStart` _item)
  (if (!= (`self.CurrentPlayer`) null)
    (`/Game/Blueprints/BP_RTS_PlayerStart.PlayerSpawned` _item (`self.CurrentPlayer`))))

(event `self.K2_PostLogin`
  (params (NewPlayer :type "PlayerController Object Reference"))
  (set `self.CurrentPlayer` NewPlayer))

(fn `RegisterTeam`
  (params (NewTeam :type "/Game/Blueprints/BP_RTS_TeamState Object Reference"))
  (returns (TeamIndex :type Byte))
  (bind _teams (`self.Teams`))
  (if (== (`KismetArrayLibrary.Array_Find` _teams NewTeam) -1)
    (bind _returnvalue (`KismetArrayLibrary.Array_Add` _teams NewTeam))
    (return (`KismetMathLibrary.Conv_IntToByte` _returnvalue))))

(fn `UserConstructionScript`)