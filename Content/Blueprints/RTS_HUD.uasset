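; RTS HUD that draws a building icon with a hit box and runs the mouse-following building placement preview.
; Clicking the icon spawns a collision-free Building_Master in preview mode and opens a Tick gate, which CloseTickGate shuts.
; DrawHUD deprojects the cursor for Tick's line trace, whose hit passes through GridPlacement to move the preview.
; Tick also writes that location and the build-mode flag to MyController.
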(event `self.ReceiveTick`
  (params (DeltaSeconds :type "Float (single-precision)"))
  (bind _mycontroller (`self.MyController`))
  (bind _deproject_worldlocation (`self.Deproject_WorldLocation`))
  ;[1 1 1] Spawn a preview mesh so it moves with the mouse.
  (`/Engine/EditorBlueprintResources/StandardMacros.Gate` true :!label _label
    (:`Exit`
      (bind _outhit (`KismetSystemLibrary.LineTraceSingle` _deproject_worldlocation (+ _deproject_worldlocation (* (`self.Deproject_WorldDirection`) 5000.0)) "TraceTypeQuery1"))
      (`|ExecutionSequence`
        (:`then_0`
          (bind _returnvalue (`KismetMathLibrary.MakeVector` (`/Game/Libraries/RTS_Macro_Library.GridSnap` (.x (`.ImpactPoint` (`GameplayStatics.BreakHitResult` _outhit)))) (`/Game/Libraries/RTS_Macro_Library.GridSnap` (.y (`.ImpactPoint` (`GameplayStatics.BreakHitResult` _outhit)))) (.z (`.ImpactPoint` (`GameplayStatics.BreakHitResult` _outhit)))))
          (set `/Game/Blueprints/MyController.PreviewBuildingLocation` _returnvalue _mycontroller))
        (:`then_1`
          (`self.K2_SetActorLocation` (stale `self.ReceiveHitBoxClick` _returnvalue) _returnvalue false))
        (:`then_2`
          (set `/Game/Blueprints/MyController.bIsInBuildMode` true _mycontroller))))))

(event `CloseTickGate`
  ;[1 1 1] Spawn a preview mesh so it moves with the mouse.
  (goto _label :!via `Close`))

(event `self.ReceiveHitBoxClick`
  (params (BoxName :type Name))
  ;[1 1 1] Spawn a preview mesh so it moves with the mouse.
  (switch `name` BoxName
    (:`PlaceBuilding`
      (bind _returnvalue (`|SpawnActorFromClass` "/Game/Blueprints/Building_Master.Building_Master_C" (`KismetMathLibrary.MakeTransform` (0.0 0.0 0.0))))
      (`/Game/Blueprints/Building_Master.PreviewMode` _returnvalue)
      (set `/Game/Blueprints/MyController.PreviewBuilding` _returnvalue (`self.MyController`))
      (`self.SetActorEnableCollision` _returnvalue false)
      (goto _label :!via `Open`))))

(event `self.ReceiveBeginPlay`
  ;[1 1 1] Cast and save MyController
  (bind _asmycontroller_c (cast `/Game/Blueprints/MyController` (`GameplayStatics.GetPlayerController` 0)))
  (set `self.MyController` _asmycontroller_c))

(event `self.ReceiveDrawHUD`
  (params (SizeX :type Integer) (SizeY :type Integer))
  (bind _buildingicon_position (`self.BuildingIcon_Position`))
  (bind _buildingicon (`self.BuildingIcon`))
  (bind (_locationx _locationy) (`PlayerController.GetMousePosition` (`GameplayStatics.GetPlayerController` 0)))
  (bind (_x _y) (`KismetMathLibrary.BreakVector2D` _buildingicon_position))
  (bind (_worldposition _worlddirection) (`self.Deproject` _locationx _locationy))
  (bind _returnvalue (`KismetMathLibrary.Conv_IntToDouble` (`Texture2D.Blueprint_GetSizeX` _buildingicon)))
  (bind _returnvalue_2 (`KismetMathLibrary.Conv_IntToDouble` (`Texture2D.Blueprint_GetSizeY` _buildingicon)))
  (`|ExecutionSequence`
    (:`then_0`
      (set `self.SizeX` SizeX))
    (:`then_1`
      (set `self.SizeY` SizeY))
    (:`then_2`
      (`self.AddHitBox` _buildingicon_position (`KismetMathLibrary.MakeVector2D` _returnvalue _returnvalue_2) "PlaceBuilding")
      (`self.DrawRect` (struct :`R` 0.035622 :`G` 0.223681 :`B` 0.485 :`A` 0.2) _x _y _returnvalue _returnvalue_2))
    (:`then_3`
      (`self.DrawTextureSimple` _buildingicon _x _y 1.0))
    (:`then_4`
      (set `self.Deproject_WorldLocation` _worldposition))
    (:`then_5`
      (set `self.Deproject_WorldDirection` _worlddirection))))

(fn `UserConstructionScript`)