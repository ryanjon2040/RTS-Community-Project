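; BP_ResourceSpawner scatters Wood, Gold or Food resource actors around itself for an RTS, via its SpawnResources event.
; For each requested resource, it runs a Visibility line trace between separately randomized points within SpawnRadius, with end Z scaled far out.
; Only Landscape hits spawn the actor matching ResourceType at the impact point, which then receives a random size through SetResourceSize.
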(event `SpawnResources`
  (bind _returnvalue (`NavigationSystem.GetRandomPointInRadius` (`self.K2_GetActorLocation`) (`self.SpawnRadius`)))
  (bind _returnvalue_2 (cast `/Game/ENUMS/RTS_ENUM_ResourceSize` (`KismetMathLibrary.Conv_IntToByte` (`KismetMathLibrary.RandomIntegerInRange` 0 3))))
  (for _ (range (+ (`self.NumberOfResources`) 1))
    (bind _outhit (`KismetSystemLibrary.LineTraceSingle` :`Start` _returnvalue :`End` (`KismetMathLibrary.MakeVector` (.x _returnvalue) (.y _returnvalue) (.z (* _returnvalue 10000.0))) :`TraceChannel` "TraceTypeQuery1" :`DrawDebugType` (`self.DebugDraw`)))
    (bind (_location _normal _impactpoint _impactnormal _physmat _hitactor) (`GameplayStatics.BreakHitResult` _outhit))
    (cast `Landscape` _hitactor)
    (switch `/Game/ENUMS/RTS_ENUM_ResourceType` (`self.ResourceType`)
      (:`NewEnumerator0`
        (bind _returnvalue_3 (`KismetMathLibrary.Conv_VectorToTransform` _impactpoint))
        (bind _returnvalue_4 (`|SpawnActorFromClass` "/Game/Blueprints/Resources/BP_Wood.BP_Wood_C" _returnvalue_3))
        (set `/Game/Blueprints/BP_RTS_Resource_Master.ResourceSize` _returnvalue_2 _returnvalue_4)
        (`/Game/Blueprints/BP_RTS_Resource_Master.SetResourceSize` _returnvalue_4 (`/Game/Blueprints/BP_RTS_Resource_Master.ResourceSize` _returnvalue_4)))
      (:`NewEnumerator1`
        (bind _returnvalue_5 (`|SpawnActorFromClass` "/Game/Blueprints/Resources/BP_Gold.BP_Gold_C" _returnvalue_3))
        (set `/Game/Blueprints/BP_RTS_Resource_Master.ResourceSize` _returnvalue_2 _returnvalue_5)
        (`/Game/Blueprints/BP_RTS_Resource_Master.SetResourceSize` _returnvalue_5 (`/Game/Blueprints/BP_RTS_Resource_Master.ResourceSize` _returnvalue_5)))
      (:`NewEnumerator2`
        (bind _returnvalue_6 (`|SpawnActorFromClass` "/Game/Blueprints/Resources/BP_Food.BP_Food_C" _returnvalue_3))
        (set `/Game/Blueprints/BP_RTS_Resource_Master.ResourceSize` _returnvalue_2 _returnvalue_6)
        (`/Game/Blueprints/BP_RTS_Resource_Master.SetResourceSize` _returnvalue_6 (`/Game/Blueprints/BP_RTS_Resource_Master.ResourceSize` _returnvalue_6))))))

(fn `UserConstructionScript`)