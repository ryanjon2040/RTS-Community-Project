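; Upgrade controller for an RTS actor, tracking which upgrades its class has locked, available and active.
; Shortly after BeginPlay it finds the upgrade manager and loads its class's upgrades as locked, unlocking those whose conditions the active upgrades satisfy.
; Purchases go through the manager; successful ones activate single-use upgrades and refresh the lists, while multi-activate upgrades stay available.
; The K key buys the wood upgrade directly.
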(event EventBeginPlay
  (|CallParentFunction)
  (Utilities|FlowControl|Delay 0.2)
  (bind _outactors (Actor|GetAllActorsOfClass "/Game/Blueprints/BP_RTS_UpgradeManager.BP_RTS_UpgradeManager_C"))
  (if (> (Utilities|Array|Length _outactors) 0)
    (bind _asbp_rts_upgrademanager_c (Utilities|Casting|CastToBP_RTS_UpgradeManager (Utilities|Array|Get(acopy) _outactors)))
    (Variables|Upgrades|SetUpgradeManager _asbp_rts_upgrademanager_c)
    (bind _asactor (Utilities|Casting|CastToActorClass (Utilities|GetClass self)))
    (bind _upgrades (Default|GetUpgradesforClass (Variables|Upgrades|GetUpgradeManager) _asactor))
    (Variables|Upgrades|SetLockedUpgrades _upgrades)
    (CallFunction|UpdateUpgradeLists)))

(event Input|KeyboardEvents|K
  (:Pressed
    (if (!= (Variables|Upgrades|GetUpgradeManager) 0)
      (bind _array_element (Utilities|Array|ForEachLoopwithBreak (Variables|Upgrades|GetAvailableUpgrades) :!label _label)
        (:LoopBody
          (if (== (Utilities|GetClass _array_element) "/Game/Blueprints/Upgrades/U_AddWood.U_AddWood_C")
            (CallFunction|BuyUpgrade _array_element)
            (goto _label Break)))))))

(fn ConstructionScript
  (|CallParentFunction))

(fn UpdateUpgradeLists
  (Utilities|FlowControl|Sequence
    (:then_0
      (for _array_element (Variables|Upgrades|GetActiveUpgrades)
        (bind _asbp_rts_upgrade_master_c (Utilities|Casting|CastToBP_RTS_Upgrade_MasterClass (Utilities|GetClass _array_element)))
        (Utilities|Array|Add (LocalVariables|GetMyUpgrades) _asbp_rts_upgrade_master_c)))
    (:then_1
      (for _array_element_2 (Variables|Upgrades|GetLockedUpgrades)
        (bind _bunlocked (Default|ShouldbeUnlocked _array_element_2 (LocalVariables|GetMyUpgrades)))
        (if _bunlocked
          (Utilities|Array|Add (LocalVariables|GetNewUpgrades) _array_element_2))))
    (:then_2
      (for _array_element_3 (LocalVariables|GetNewUpgrades)
        (Utilities|Array|Add (Variables|Upgrades|GetAvailableUpgrades) _array_element_3)
        (Utilities|Array|RemoveItem (Variables|Upgrades|GetLockedUpgrades) _array_element_3)))
    (:then_3
      (return))))

(fn BuyUpgrade
  (params (RequestedUpgrade :type BP%20RTS%20Upgrade%20Master%20Object%20Reference))
  (bind _self self)
  (bind _bsucces (Default|RequestUpgrade (Variables|Upgrades|GetUpgradeManager) RequestedUpgrade _self _self))
  (if _bsucces
    (Utilities|FlowControl|Sequence
      (:then_0
        (if (not (Variables|/Game/Blueprints/BP_RTS_Upgrade_Master.BP_RTS_Upgrade_Master_C|GetbMultiActivate RequestedUpgrade))
          (Utilities|Array|Add (Variables|Upgrades|GetActiveUpgrades) RequestedUpgrade)
          (Utilities|Array|RemoveItem (Variables|Upgrades|GetAvailableUpgrades) RequestedUpgrade)))
      (:then_1
        (CallFunction|UpdateUpgradeLists)))))