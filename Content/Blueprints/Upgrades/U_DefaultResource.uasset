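; U_DefaultResource is an RTS upgrade Blueprint that handles the gold, wood and food cost of an upgrade.
; HasEnoughResources reads the BP_RTS_GameState totals and returns true only when all three cover their costs.
; DepleteResources calls the parent implementation, then subtracts each cost through the game state's Update functions.
; Both use the shared game state, so the Controller and Owner inputs do not select whose resources are used.
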(event EventDepleteResources
  (params (Owner :type BP%20RTS%20Controller%20Object%20Reference))
  (|CallParentFunction Owner)
  (bind _asbp_rts_gamestate_c (Utilities|Casting|CastToBP_RTS_GameState (Game|GetGameState)))
  (Default|UpdateGold _asbp_rts_gamestate_c (* (Variables|Default|GetGoldCost) -1))
  (Default|UpdateWood _asbp_rts_gamestate_c (* (Variables|Default|GetWoodCost) -1))
  (Default|UpdateFood _asbp_rts_gamestate_c (* (Variables|Default|GetFoodCost) -1)))

(fn ConstructionScript
  (|CallParentFunction))

(fn HasEnoughResources
  (params (Controller :type BP%20RTS%20Controller%20Object%20Reference))
  (Utilities|FlowControl|Sequence
    (:then_0
      (bind _asbp_rts_gamestate_c (Utilities|Casting|CastToBP_RTS_GameState (Game|GetGameState)))
      (LocalVariables|SetbHasEnough (Math|Boolean|ANDBoolean (>= (Variables|/Game/Blueprints/BP_RTS_GameState.BP_RTS_GameState_C|GetGold _asbp_rts_gamestate_c) (Variables|Default|GetGoldCost)) (>= (Variables|/Game/Blueprints/BP_RTS_GameState.BP_RTS_GameState_C|GetWood _asbp_rts_gamestate_c) (Variables|Default|GetWoodCost)) (>= (Variables|/Game/Blueprints/BP_RTS_GameState.BP_RTS_GameState_C|GetFood _asbp_rts_gamestate_c) (Variables|Default|GetFoodCost)))))
    (:then_1
      (return (LocalVariables|GetbHasEnough)))))