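; RTS upgrade manager that holds the game's upgrades and handles purchase requests for them.
; On BeginPlay it spawns an actor for each configured upgrade class and stores those deriving from BP_RTS_Upgrade_Master.
; GetUpgradesForClass filters them by valid actor list, treating an empty list as available to every class.
; RequestUpgrade delegates the buyer's resource check and the activation to the upgrade itself, then returns whether it was bought.
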(event EventBeginPlay
  (for _array_element (Variables|Default|GetUpgradeClasses)
    (bind _returnvalue (Game|SpawnActorfromClass _array_element (Math|Transform|MakeTransform "0, 0, 0") false))
    (bind _asbp_rts_upgrade_master_c (Utilities|Casting|CastToBP_RTS_Upgrade_Master _returnvalue))
    (Utilities|Array|Add (Variables|Default|GetUpgrades) _asbp_rts_upgrade_master_c)))

(fn ConstructionScript)

(fn GetUpgradesforClass
  (params (Class :type Actor%20Class%20Reference))
  (for _array_element (Variables|Default|GetUpgrades)
    (if (or (Utilities|Array|ContainsItem (Variables|/Game/Blueprints/BP_RTS_Upgrade_Master.BP_RTS_Upgrade_Master_C|GetValidActorList _array_element) Class) (== (Utilities|Array|Length (Variables|/Game/Blueprints/BP_RTS_Upgrade_Master.BP_RTS_Upgrade_Master_C|GetValidActorList _array_element)) 0))
      (Utilities|Array|Add (LocalVariables|GetAvailableUpgrades) _array_element)))
  (return (LocalVariables|GetAvailableUpgrades)))

(fn RequestUpgrade
  (params (RequestedUpgrade :type BP%20RTS%20Upgrade%20Master%20Object%20Reference) (Buyer :type BP%20RTS%20Controller%20Object%20Reference) (Instigator :type Actor%20Object%20Reference))
  (Utilities|FlowControl|Sequence
    (:then_0
      (bind _enoughresources (Default|HasEnoughResources RequestedUpgrade Buyer))
      (if _enoughresources
        (Default|Activate RequestedUpgrade Instigator Buyer)
        (LocalVariables|SetbBought true)))
    (:then_1
      (return (LocalVariables|GetbBought)))))