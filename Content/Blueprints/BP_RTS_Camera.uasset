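; RTS camera rig that pans across the world and zooms along a boom arm.
; Tick moves the root without sweep from move-axis variables, rotated by the root's yaw and doubled in speed while Left Shift is held; the step is not scaled by delta time.
; ZoomIn and ZoomOut set a clamped target arm length that Tick eases toward.
; The construction script applies initial arm length, projection mode, FOV and ortho width.
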(event `self.ReceiveTick`
  (params (DeltaSeconds :type "Float (single-precision)"))
  (bind _mainroot (`self.MainRoot`))
  (bind _cameramovementspeed (`self.CameraMovementSpeed`))
  (bind _cameraboom (`self.CameraBoom`))
  ;[1 1 1] Zoom Interp
  (set `SpringArmComponent.TargetArmLength` (`KismetMathLibrary.FInterpTo` (`SpringArmComponent.TargetArmLength` _cameraboom) (`self.CameraBoomLength`) DeltaSeconds (`self.CameraZoomSpeed`)) _cameraboom)
  ;[1 1 1] Camera WASD Movement
  (set `self.CameraPan` (`KismetMathLibrary.MakeVector` (`self.MoveForward_AXIS`) (`self.MoveRight_AXIS`)))
  (set `self.CameraPan` (* (`KismetMathLibrary.GreaterGreater_VectorRotator` (`self.CameraPan`) (`KismetMathLibrary.MakeRot` 0.0 (.yaw (`SceneComponent.K2_GetComponentRotation` _mainroot)))) (`KismetMathLibrary.SelectFloat` (* _cameramovementspeed 2.0) _cameramovementspeed (`PlayerController.IsInputKeyDown` (`GameplayStatics.GetPlayerController` 0) "LeftShift"))))
  (`SceneComponent.SetWorldLocation` _mainroot (+ (`SceneComponent.K2_GetComponentLocation` _mainroot) (`self.CameraPan`)) false))

(event `ZoomIn`
  ;[1 1 1] Zoom Events
  (set `self.CameraBoomLength` (`KismetMathLibrary.FClamp` (- (`SpringArmComponent.TargetArmLength` (`self.CameraBoom`)) 300.0) 0.0 4000.0)))

(event `ZoomOut`
  ;[1 1 1] Zoom Events
  (set `self.CameraBoomLength` (`KismetMathLibrary.FClamp` (+ (`SpringArmComponent.TargetArmLength` (`self.CameraBoom`)) 300.0) 0.0 4000.0)))

(fn `UserConstructionScript`
  (bind _rts_camera (`self.RTS_Camera`))
  (set `SpringArmComponent.TargetArmLength` (`self.CameraBoomLength`) (`self.CameraBoom`))
  (set `CameraComponent.ProjectionMode` (`self.ProjectionMode`) _rts_camera)
  (set `CameraComponent.FieldOfView` (`self.FOV`) _rts_camera)
  (set `CameraComponent.OrthoWidth` (`self.OrthograhicWidth`) _rts_camera))