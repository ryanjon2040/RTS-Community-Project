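; BP_Arrow_Curve is a short-lived animated arrow effect built from four arrow meshes set at 90-degree yaw steps.
; On BeginPlay, the Arrow_Animation timeline drives a shared pitch value, updating all four meshes' relative rotations each tick with fixed yaw and flipped roll.
; When the timeline finishes, the actor destroys itself.
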(event `self.ReceiveBeginPlay`
  (bind (_direction _pitch) (`Timeline|Arrow_Animation` :!via `PlayFromStart`)
    (:`Update`
      (`|ExecutionSequence`
        (:`then_0`
          (`SceneComponent.SetRelativeRotation` (`self.ArrowMesh1`) (`KismetMathLibrary.MakeRot` _pitch 0.0 -180.0) false))
        (:`then_1`
          (`SceneComponent.SetRelativeRotation` (`self.ArrowMesh2`) (`KismetMathLibrary.MakeRot` _pitch 90.0 180.0) false))
        (:`then_2`
          (`SceneComponent.SetRelativeRotation` (`self.ArrowMesh3`) (`KismetMathLibrary.MakeRot` _pitch -180.0 -180.0) false))
        (:`then_3`
          (`SceneComponent.SetRelativeRotation` (`self.ArrowMesh4`) (`KismetMathLibrary.MakeRot` _pitch -90.0 -180.0) false))))
    (:`Finished`
      (`self.K2_DestroyActor`))))

(fn `UserConstructionScript`)