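; RTS building placement preview actor that shows a ghost mesh of the selected building, configured by Activate and cleared by DeActivate.
; While active, Tick snaps it to the owning controller's grid under the cursor.
; Placement is valid without overlapping I_Interaction actors, with cursor normal Y within the slope limit, and with enough game-state resources.
; SetMaterial swaps six material slots between preview and error materials only when validity changes.
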(event Custom|SetMaterial
  (params (bValid :type Boolean))
  (if (not (Math|Boolean|Equal(Boolean) bValid (Variables|Default|GetbValidLocation)))
    (Variables|Default|SetbValidLocation bValid)
    (if (Variables|Default|GetbValidLocation)
      ;[1 1 1] Set materials accordingly
      (Rendering|Material|SetMaterial (Variables|Default|GetStaticMesh) 0 "/Game/Materials/M_PreviewMode.M_PreviewMode")
      ;[1 1 1] Because barracks has a lot of materials :)
      (Rendering|Material|SetMaterial (Variables|Default|GetStaticMesh) 1 "/Game/Materials/M_PreviewMode.M_PreviewMode")
      (Rendering|Material|SetMaterial (Variables|Default|GetStaticMesh) 2 "/Game/Materials/M_PreviewMode.M_PreviewMode")
      (Rendering|Material|SetMaterial (Variables|Default|GetStaticMesh) 3 "/Game/Materials/M_PreviewMode.M_PreviewMode")
      (Rendering|Material|SetMaterial (Variables|Default|GetStaticMesh) 4 "/Game/Materials/M_PreviewMode.M_PreviewMode")
      (Rendering|Material|SetMaterial (Variables|Default|GetStaticMesh) 5 "/Game/Materials/M_PreviewMode.M_PreviewMode")
      (else
        (Rendering|Material|SetMaterial (Variables|Default|GetStaticMesh) 0 "/Game/Materials/M_PreviewMode_Error.M_PreviewMode_Error")
        (Rendering|Material|SetMaterial (Variables|Default|GetStaticMesh) 1 "/Game/Materials/M_PreviewMode_Error.M_PreviewMode_Error")
        (Rendering|Material|SetMaterial (Variables|Default|GetStaticMesh) 2 "/Game/Materials/M_PreviewMode_Error.M_PreviewMode_Error")
        (Rendering|Material|SetMaterial (Variables|Default|GetStaticMesh) 3 "/Game/Materials/M_PreviewMode_Error.M_PreviewMode_Error")
        (Rendering|Material|SetMaterial (Variables|Default|GetStaticMesh) 4 "/Game/Materials/M_PreviewMode_Error.M_PreviewMode_Error")
        (Rendering|Material|SetMaterial (Variables|Default|GetStaticMesh) 5 "/Game/Materials/M_PreviewMode_Error.M_PreviewMode_Error")))))

(event Custom|Activate
  (params (TargetClass :type BP%20Building%20Master%20Class%20Reference) (TargetCost :type BP%20RTS%20Resources%20Structure) (Mesh :type Static%20Mesh%20Object%20Reference) (TargetProxyClass :type BP%20Construction%20Proxy%20Class%20Reference))
  (bind _staticmesh (Variables|Default|GetStaticMesh))
  ;[1 1 1] Initialization
  (Variables|Default|SetProxyClass TargetProxyClass)
  (Variables|Default|SetBuildingClass TargetClass)
  (Variables|Default|SetResourceCost TargetCost)
  (Variables|Default|SetbIsActive true)
  (Components|StaticMesh|SetStaticMesh _staticmesh Mesh)
  (Variables|Default|SetExtent (.BoxExtent (Collision|GetComponentBounds _staticmesh)))
  (CallFunction|SetMaterial true))

(event Custom|DeActivate
  (Variables|Default|SetProxyClass 0)
  (Variables|Default|SetBuildingClass 0)
  (Variables|Default|SetResourceCost "")
  (Variables|Default|SetbIsActive false)
  (Components|StaticMesh|SetStaticMesh (Variables|Default|GetStaticMesh) 0)
  (Variables|Default|SetExtent "0, 0, 0"))

(event EventTick
  (params (DeltaSeconds :type Float%20%28single-precision%29))
  (bind _ownerpc (Variables|Default|GetOwnerPC))
  (bind _ownerpc_2 (Variables|Default|GetOwnerPC))
  (bind _resourcecost (Variables|Default|GetResourceCost))
  (bind _cursorworldlocation (Variables|/Game/Blueprints/BP_RTS_Controller.BP_RTS_Controller_C|GetCursorWorldLocation _ownerpc))
  (bind _gridsize (Variables|/Game/Blueprints/BP_RTS_Controller.BP_RTS_Controller_C|GetGridSize _ownerpc))
  (bind (_x _y _z) (Math|Vector|BreakVector _cursorworldlocation))
  (if (and (!= (Variables|Default|GetOwnerPC) 0) (Variables|Default|GetbIsActive))
    (Utilities|FlowControl|Sequence
      (:then_0
        ;[1 1 1] Set location on grid
        (Transformation|SetActorLocation (Math|Vector|MakeVector (Utilities|GridSnap _x _gridsize) (Utilities|GridSnap _y _gridsize) _z) false))
      (:then_1
        (bind _bcontinue (CallFunction|CheckOverlappingActors))
        (if _bcontinue
          (if (> (Math|Float|Absolute(Float) (.Y (Math|Vector|BreakVector (Variables|/Game/Blueprints/BP_RTS_Controller.BP_RTS_Controller_C|GetCursorWorldNormal _ownerpc_2)))) (Variables|/Game/Blueprints/BP_RTS_Controller.BP_RTS_Controller_C|GetMaxBuildSlope _ownerpc_2))
            (CallFunction|SetMaterial false :!label _label)
            (else
              (bind _asbp_rts_gamestate_c (Utilities|Casting|CastToBP_RTS_GameState (Game|GetGameState))
                (:then
                  (if (Math|Boolean|ANDBoolean (>= (.wood (Variables|/Game/Blueprints/BP_RTS_GameState.BP_RTS_GameState_C|GetResources _asbp_rts_gamestate_c)) (.wood _resourcecost)) (>= (.gold (Variables|/Game/Blueprints/BP_RTS_GameState.BP_RTS_GameState_C|GetResources _asbp_rts_gamestate_c)) (.gold _resourcecost)) (>= (.food (Variables|/Game/Blueprints/BP_RTS_GameState.BP_RTS_GameState_C|GetResources _asbp_rts_gamestate_c)) (.food _resourcecost)) (>= (.knowledge (Variables|/Game/Blueprints/BP_RTS_GameState.BP_RTS_GameState_C|GetResources _asbp_rts_gamestate_c)) (.knowledge _resourcecost)) (>= (.skill (Variables|/Game/Blueprints/BP_RTS_GameState.BP_RTS_GameState_C|GetResources _asbp_rts_gamestate_c)) (.skill _resourcecost)))
                    (CallFunction|SetMaterial true)
                    (else
                      (goto _label))))
                (:CastFailed
                  (goto _label)))))
          (else
            (goto _label)))))))

(fn ConstructionScript)

(fn CheckOverlappingActors
  (bind _overlappingactors (Collision|GetOverlappingActors "/Script/Engine.Actor" :!class /Script/Engine.Actor))
  ;[1 1 1] Continue if overlapping actors don't implement I_Interaction, so currently you can place buildings in static meshes
  (LocalVariables|SetbShouldContinue true)
  (if (> (Utilities|Array|Length _overlappingactors) 0)
    (bind _array_element (Utilities|Array|ForEachLoopwithBreak _overlappingactors :!label _label)
      (:LoopBody
        (if (Utilities|DoesObjectImplementInterface _array_element "/Game/Blueprints/I_Interaction.I_Interaction_C")
          (LocalVariables|SetbShouldContinue false)
          (goto _label Break)))
      (:Completed
        (return (LocalVariables|GetbShouldContinue))))
    (else
      (return (LocalVariables|GetbShouldContinue)))))