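; Team state actor for an RTS that tracks one team's index, color, characters and buildings.
; On BeginPlay it registers itself with BP_RTS_Game, which returns its team index, and picks a team color from the default colors by that index.
; Add and remove events keep the unit lists free of duplicates, and HasLostEverything reports when both lists are empty.
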(event `self.ReceiveBeginPlay`
  (bind _asbp_rts_game_c (cast `/Game/Blueprints/BP_RTS_Game` (`GameplayStatics.GetGameMode`)))
  (bind _teamindex (`/Game/Blueprints/BP_RTS_Game.RegisterTeam` _asbp_rts_game_c self))
  (`self.SetTeamIndex` _teamindex))

(event `SetTeamIndex`
  (params (NewTeamIndex :type Byte))
  (set `self.TeamIndex` NewTeamIndex)
  (if (and (>= NewTeamIndex 0) (< NewTeamIndex (`KismetMathLibrary.Conv_IntToByte` (`KismetArrayLibrary.Array_Length` (`self.DefaultColors`)))))
    (set `self.TeamColor` (`KismetArrayLibrary.Array_Get` (`self.DefaultColors`) (`KismetMathLibrary.Conv_ByteToInt` NewTeamIndex)))))

(event `AddCharacter`
  (params (Character :type "/Game/Blueprints/BP_RTS_Character Object Reference"))
  (bind _characters (`self.Characters`))
  (if (== (`KismetArrayLibrary.Array_Find` _characters Character) -1)
    (`KismetArrayLibrary.Array_Add` _characters Character)))

(event `RemoveCharacter`
  (params (Character :type "/Game/Blueprints/BP_RTS_Character Object Reference"))
  (bind _characters (`self.Characters`))
  (if (!= (`KismetArrayLibrary.Array_Find` _characters Character) -1)
    (`KismetArrayLibrary.Array_RemoveItem` _characters Character)))

(event `AddBuilding`
  (params (Building :type "/Game/Blueprints/BP_Building_Master Object Reference"))
  (bind _buildings (`self.Buildings`))
  (if (== (`KismetArrayLibrary.Array_Find` _buildings Building) -1)
    (`KismetArrayLibrary.Array_Add` _buildings Building)))

(event `RemoveBuilding`
  (params (Building :type "/Game/Blueprints/BP_Building_Master Object Reference"))
  (bind _buildings (`self.Buildings`))
  (if (!= (`KismetArrayLibrary.Array_Find` _buildings Building) -1)
    (`KismetArrayLibrary.Array_RemoveItem` _buildings Building)))

(fn `HasLostEverything`
  (returns (bHasLostEverything :type Boolean))
  (return (and (<= (`KismetArrayLibrary.Array_Length` (`self.Characters`)) 0) (<= (`KismetArrayLibrary.Array_Length` (`self.Buildings`)) 0))))

(fn `UserConstructionScript`)