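; RTS player start that sets up a player's starting base and ownership when that player spawns.
; PlayerSpawned spawns a headquarters at the start's location and rotation, even if colliding, and adds it to the starting buildings list.
; If the controller has a PlayerState, it assigns that state to every starting building and unit, also initializing each building.
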(event `PlayerSpawned`
  (params (PC :type "PlayerController Object Reference"))
  (bind _playerstate (`Controller.PlayerState` PC))
  (`|ExecutionSequence`
    (:`then_0`
      (bind _returnvalue (`|SpawnActorFromClass` "/Game/Blueprints/Structures/Headquarters/BP_Headquarters.BP_Headquarters_C" (`KismetMathLibrary.MakeTransform` (`self.K2_GetActorLocation`) (`self.K2_GetActorRotation`)) true))
      (`KismetArrayLibrary.Array_Add` (`self.StartingBuildings`) _returnvalue))
    (:`then_1`
      (if (!= _playerstate null)
        (`|ExecutionSequence`
          (:`then_0`
            (for _array_element (`self.StartingBuildings`)
              (`/Game/Blueprints/BP_Building_Master.SetPlayerState` _array_element _playerstate)
              (`/Game/Blueprints/BP_Building_Master.Initialize` _array_element)))
          (:`then_1`
            (for _array_element_2 (`self.StartingUnits`)
              (`/Game/Blueprints/BP_RTS_Character.SetPlayerState` _array_element_2 _playerstate))))))))

(fn `UserConstructionScript`)