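; MyCharacter is a character Blueprint with a selection decal that shows when a controller takes possession of it.
; The decal starts hidden on BeginPlay, and the PossessMe event calls Possess on the supplied controller, then reveals it through ToggleSelectionDecal.
; The construction script scales the decal uniformly from the mesh's bounding sphere radius minus a fixed offset.
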(event `self.ReceiveBeginPlay`
  (`self.ToggleSelectionDecal` true))

(event `PossessMe`
  (params (MyController :type "/Game/Blueprints/MyController Object Reference"))
  (`Controller.Possess` MyController null)
  (`self.ToggleSelectionDecal` false))

(fn `ToggleSelectionDecal`
  (params (bHideDecal :type Boolean))
  (`SceneComponent.SetHiddenInGame` (`self.SelectionDecal`) bHideDecal false))

(fn `UserConstructionScript`
  (`SceneComponent.SetRelativeScale3D` (`self.SelectionDecal`) (`KismetMathLibrary.Conv_DoubleToVector` (- (`.SphereRadius` (`KismetSystemLibrary.GetComponentBounds` (`self.Mesh`))) 180.0))))