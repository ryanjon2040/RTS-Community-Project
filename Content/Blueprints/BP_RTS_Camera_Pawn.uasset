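; RTS camera pawn with edge-of-screen and key-axis panning, zoom, and yaw rotation while a rotation-mode action is held.
; Inputs set TargetGodLocation, kept within min/max distance of the traced ground; zoom snaps, while Tick interpolates pans.
; Curves over distance ratio scale pan and zoom speed and optionally auto-tilt the spring arm.
; Rotation only yaws the actor, as the pivot-orbit move in RotateCameraByAngle is disconnected.
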(event Custom|Move
  (params (Forward :type Float%20%28single-precision%29) (Right :type Float%20%28single-precision%29))
  ;[1 1 1] Screen movement
  (Utilities|HasMovementInput Forward Right
    (:Yes
      (if (not (Variables|Default|GetbInRotationMode))
        (bind _next_location (CallFunction|CalculateNextLocationfromInputs Forward Right))
        (CallFunction|MoveCameratoLocation _next_location true)))))

(event EventTick
  (params (DeltaSeconds :type Float%20%28single-precision%29))
  (bind _returnvalue (Viewport|GetViewportSize))
  (bind _returnvalue_2 (Viewport|GetViewportSize))
  (bind _returnvalue_3 (Viewport|GetViewportSize))
  (bind _returnvalue_4 (Viewport|GetViewportSize))
  (bind _returnvalue_5 (Transformation|GetActorLocation))
  (bind _targetgodlocation (Variables|Default|GetTargetGodLocation))
  (bind _targetgodlocation_2 (Variables|Default|GetTargetGodLocation))
  (bind _targetgodlocation_3 (Variables|Default|GetTargetGodLocation))
  (bind _springarm (Variables|Default|GetSpringArm))
  (bind _returnvalue_6 (- _returnvalue_5 _targetgodlocation_2))
  (bind _relativerotation (Variables|/Script/Engine.SceneComponent|GetRelativeRotation _springarm))
  (bind _returnvalue_7 (Math|Vector|VectorLength _returnvalue_6))
  (bind (_pitch _yaw _roll) (Class|KismetMathLibrary|BreakRot _relativerotation))
  (bind _returnvalue_8 (Math|Float|Absolute(Float) _returnvalue_7))
  ;[1 1 1] Tick and Interpolation
  (Utilities|FlowControl|Sequence
    (:then_0
      (bind _outhit (Collision|LineTraceByChannel _targetgodlocation_3 (+ _targetgodlocation_3 (* (Math|Rotator|GetRotationXVector (Transformation|GetWorldRotation (Variables|Default|GetCamera))) (Variables|Default|GetMaxTraceDistance))) "TraceTypeQuery3" false 0 "None"))
      (if (Math|Vector|NotEqual(Vector) (.Location (Collision|BreakHitResult _outhit)) "0, 0, 0" 0.0)
        (Variables|Default|SetTraceHitLocation (.Location (Collision|BreakHitResult _outhit)))
        (Variables|Default|SetDesiredCameraDistance (Math|Vector|VectorLength (- (Transformation|GetActorLocation) (.Location (Collision|BreakHitResult _outhit)))))))
    (:then_1
      (if (not (Variables|Default|GetbInRotationMode))
        (if (> _returnvalue_8 (Variables|Default|GetInterpTolerance))
          (Transformation|SetActorLocation (Math|Interpolation|VInterpTo (Transformation|GetActorLocation) _targetgodlocation DeltaSeconds 1e+01) false)
          (CallFunction|UpdatePivotCache :!label _label)
          (Variables|Default|SetApproximateCameraDistance (Math|Float|Absolute(Float) (Math|Vector|VectorLength (- (Transformation|GetActorLocation) (Variables|Default|GetCachedRotationPivot)))))
          (if (Variables|Default|GetAutoTiltBasedOnZoom)
            (Transformation|SetRelativeRotation _springarm (Class|KismetMathLibrary|MakeRot (Math|Curves|GetFloatValue (Variables|Default|GetTiltVsDistanceCurve) (Utilities|GetDistanceRatio)) _yaw _roll) false))
          (elif (> _returnvalue_8 0.001)
            (Transformation|SetActorLocation _targetgodlocation false)
            (goto _label)))))
    (:then_2
      ;[1 1 1] Screen movement
      (bind _asplayer_controller (Utilities|Casting|CastToPlayerController (Pawn|GetController)))
      (bind (_posx _posy) (Class|VictoryBPFunctionLibrary|ViewportGetMousePosition _asplayer_controller))
      (if (and (>= _posx 0.0) (>= _posy 0.0))
        (Utilities|FlowControl|Sequence
          (:then_0
            (if (<= _posx (* (.x _returnvalue_3) 0.1))
              (CallFunction|Move 0.0 (* -1 (/ _posx (.x _returnvalue_3))))))
          (:then_1
            (if (>= _posx (* (.x _returnvalue_4) 0.9))
              (CallFunction|Move 0.0 (/ _posx (.x _returnvalue_4)))))
          (:then_2
            (if (<= _posy (* (.y _returnvalue_2) 0.1))
              (CallFunction|Move (/ _posy (.y _returnvalue_2)) 0.0)))
          (:then_3
            (if (>= _posy (* (.y _returnvalue) 0.9))
              (CallFunction|Move (* -1 (/ _posy (.y _returnvalue))) 0.0))))))))

(event EventBeginPlay
  (bind _tiltangle (Variables|Default|GetTiltAngle))
  (bind _initialcameradistance (Variables|Default|GetInitialCameraDistance))
  ;[1 1 1] Initialization
  (Variables|Default|SetTraceHitLocation (Transformation|GetActorLocation))
  (Transformation|SetRelativeRotation (Variables|Default|GetSpringArm) (Class|KismetMathLibrary|MakeRot _tiltangle 0.0 0.0) false)
  (Variables|Default|SetTargetTiltAngle _tiltangle)
  (Variables|Default|SetDesiredCameraDistance _initialcameradistance)
  (Variables|Default|SetApproximateCameraDistance _initialcameradistance)
  (CallFunction|MoveCameratoDistance _initialcameradistance false 0.0 false))

(event Input|ActionEvents|InputActionCameraZoomIn
  ;[1 1 1] Zooming
  (:Pressed
    (if (> (- (Variables|Default|GetDesiredCameraDistance) (Variables|Default|GetMinCameraDistance)) 2e+01)
      (Utilities|MergeZoomInputs (stale Input|AxisEvents|InputAxisZoom AxisValue)) ; enters at ZoomInPressed
    )))

(event Input|ActionEvents|InputActionCameraZoomOut
  ;[1 1 1] Zooming
  (:Pressed
    (if (> (- (Variables|Default|GetMaxCameraDistance) (Variables|Default|GetDesiredCameraDistance)) 1.2e+02)
      (Utilities|MergeZoomInputs (stale Input|AxisEvents|InputAxisZoom AxisValue)) ; enters at ZoomOutPressed
    )))

(event Input|ActionEvents|InputActionRotationModeTrigger
  ;[1 1 1] Rotation
  (:Pressed
    (Variables|Default|SetbInRotationMode true))
  (:Released
    (Variables|Default|SetbInRotationMode false)
    (Variables|Default|SetbIsCachedPivotValid false)))

(event Input|AxisEvents|InputAxisZoom
  (params (AxisValue :type Float%20%28single-precision%29))
  ;[1 1 1] Zooming
  (bind _effective_zoom (Utilities|MergeZoomInputs AxisValue)
    (:Exec
      (if (not (Variables|Default|GetbInRotationMode))
        (if (> (Math|Float|Absolute(Float) _effective_zoom) 0.0)
          (Variables|Default|SetDesiredCameraDistance (Math|Float|Min(Float) (Math|Float|Max(Float) (+ (* _effective_zoom (Math|Curves|GetFloatValue (Variables|Default|GetSpeedVsDistanceCurve) (Utilities|GetDistanceRatio)) 3e+01) (Variables|Default|GetApproximateCameraDistance)) (Variables|Default|GetMinCameraDistance)) (Variables|Default|GetMaxCameraDistance)))
          (CallFunction|MoveCameratoDistance (Math|Float|Min(Float) (Math|Float|Max(Float) (+ (* _effective_zoom (Math|Curves|GetFloatValue (Variables|Default|GetSpeedVsDistanceCurve) (Utilities|GetDistanceRatio)) 3e+01) (Variables|Default|GetApproximateCameraDistance)) (Variables|Default|GetMinCameraDistance)) (Variables|Default|GetMaxCameraDistance)) false 0.0 true))))))

(event Input|AxisEvents|InputAxisMoveForward
  (params (AxisValue :type Float%20%28single-precision%29))
  ;[1 1 1] WASD Movement
  (Utilities|HasMovementInput AxisValue (stale Input|AxisEvents|InputAxisMoveRight AxisValue)
    (:Yes
      (if (not (Variables|Default|GetbInRotationMode))
        (bind _next_location (CallFunction|CalculateNextLocationfromInputs AxisValue (stale Input|AxisEvents|InputAxisMoveRight AxisValue)))
        (CallFunction|MoveCameratoLocation _next_location true)))))

(event Input|AxisEvents|InputAxisMoveRight
  (params (AxisValue :type Float%20%28single-precision%29))
  ;[1 1 1] WASD Movement
  (Utilities|HasMovementInput (stale Input|AxisEvents|InputAxisMoveForward AxisValue) AxisValue
    (:Yes
      (if (not (Variables|Default|GetbInRotationMode))
        (bind _next_location (CallFunction|CalculateNextLocationfromInputs (stale Input|AxisEvents|InputAxisMoveForward AxisValue) AxisValue))
        (CallFunction|MoveCameratoLocation _next_location true)))))

(event Input|AxisEvents|InputAxisCameraRotation
  (params (AxisValue :type Float%20%28single-precision%29))
  ;[1 1 1] Rotation
  (if (and (not (Variables|Default|GetbInAxisRotation)) (Variables|Default|GetbInRotationMode))
    (CallFunction|ProcessRotationInput AxisValue)
    (else
      (Variables|Default|SetbInRotationMode false)
      (Variables|Default|SetbIsCachedPivotValid false))))

(fn ConstructionScript)

(fn MoveCameratoDistance
  (params (Distance :type Float%20%28single-precision%29) (bInterpolate :type Boolean) (InterpolationRate :type Float%20%28single-precision%29) (bConstraintDistance :type Boolean))
  (Variables|Default|SetDesiredCameraDistance Distance)
  (bind (_safelocation _distance) (CallFunction|CalculateSafeGodLocation (Variables|Default|GetTargetGodLocation) Distance bConstraintDistance))
  (Variables|Default|SetTargetGodLocation _safelocation)
  (if (not bInterpolate)
    (Variables|Default|SetApproximateCameraDistance _distance)
    (Transformation|SetActorLocation _safelocation false)))

(fn CalculateSafeGodLocation
  (params (FocalPoint :type Vector) (CameraDistance :type Float%20%28single-precision%29) (bContraintDistance :type Boolean))
  (if bContraintDistance
    (LocalVariables|SetConstrainedDistance (Math|Float|Max(Float) (Math|Float|Min(Float) CameraDistance (Variables|Default|GetMaxCameraDistance)) (Variables|Default|GetMinCameraDistance)))
    (else
      (LocalVariables|SetConstrainedDistance CameraDistance)))
  (return (+ (Variables|Default|GetTraceHitLocation) (* (* (Math|Rotator|GetRotationXVector (Transformation|GetWorldRotation (Variables|Default|GetCamera))) -1.0) (LocalVariables|GetConstrainedDistance))) (Math|Vector|VectorLength (* (* (Math|Rotator|GetRotationXVector (Transformation|GetWorldRotation (Variables|Default|GetCamera))) -1.0) (LocalVariables|GetConstrainedDistance)))))

(fn MoveCameratoLocation
  (params (Location :type Vector) (bInterpolate :type Boolean))
  (bind _camera (Variables|Default|GetCamera))
  (bind _mincameradistance (Variables|Default|GetMinCameraDistance))
  (bind _maxcameradistance (Variables|Default|GetMaxCameraDistance))
  (bind _returnvalue (Transformation|GetWorldRotation _camera))
  (bind _returnvalue_2 (Math|Rotator|GetRotationXVector _returnvalue))
  (bind _returnvalue_3 (* _returnvalue_2 -1.0))
  (bind (_outhit _returnvalue_4) (Collision|LineTraceByChannel Location (+ Location (* _returnvalue_2 (Variables|Default|GetMaxTraceDistance))) "TraceTypeQuery3" false 0 "None"))
  (if _returnvalue_4
    (if (>= (Math|Float|Absolute(Float) (Math|Vector|VectorLength (- Location (.Location (Collision|BreakHitResult _outhit))))) _mincameradistance)
      (if (<= (Math|Float|Absolute(Float) (Math|Vector|VectorLength (- Location (.Location (Collision|BreakHitResult _outhit))))) _maxcameradistance)
        (LocalVariables|SetSafe%20Location Location)
        (else
          (LocalVariables|SetSafe%20Location (+ (* _returnvalue_3 (- _maxcameradistance 1.0)) (.Location (Collision|BreakHitResult _outhit))))))
      (else
        (LocalVariables|SetSafe%20Location (+ (* _returnvalue_3 (+ _mincameradistance 1.0)) (.Location (Collision|BreakHitResult _outhit))))))
    (Variables|Default|SetTargetGodLocation (LocalVariables|GetSafe%20Location))
    (if (not bInterpolate)
      (Transformation|SetActorLocation (LocalVariables|GetSafe%20Location) true)
      (Variables|Default|SetCachedRotationPivot (.Location (Collision|BreakHitResult _outhit)))
      (Variables|Default|SetbIsCachedPivotValid false))))

(fn CalculateNextLocationfromInputs
  (params (Forward :type Float%20%28single-precision%29) (Right :type Float%20%28single-precision%29))
  (bind _returnvalue (Transformation|GetActorForwardVector))
  (bind _returnvalue_2 (Transformation|GetActorRightVector))
  (bind (_normalizedforward _normalizedright) (Utilities|NormalizeMoveInput Forward Right))
  (bind _ratio (Utilities|GetDistanceRatio))
  (bind _speedvsdistancecurve (Variables|Default|GetSpeedVsDistanceCurve))
  (bind _returnvalue_3 (* _returnvalue _normalizedforward))
  (bind _returnvalue_4 (* _returnvalue_2 _normalizedright))
  (bind _returnvalue_5 (Math|Curves|GetFloatValue _speedvsdistancecurve _ratio))
  (bind _returnvalue_6 (+ _returnvalue_3 _returnvalue_4))
  (bind _returnvalue_7 (* _returnvalue_6 _returnvalue_5))
  (Variables|Default|Setbla _returnvalue_7)
  (return (+ _returnvalue_7 (Variables|Default|GetTargetGodLocation))))

(fn ProcessRotationInput
  (params (Input :type Float%20%28single-precision%29))
  (if (Variables|Default|GetbIsCachedPivotValid)
    _
    (else
      (CallFunction|UpdatePivotCache)))
  (CallFunction|RotateCamerabyAngle (Variables|Default|GetCachedRotationPivot) (* Input (Variables|Default|GetRotationRate))))

(fn RotateCamerabyAngle
  (params (Pivot :type Vector) (Angle :type Float%20%28single-precision%29))
  (Transformation|SetActorRotation (Math|Rotator|CombineRotators (Class|KismetMathLibrary|MakeRot 0.0 Angle 0.0) (Transformation|GetActorRotation))))

(fn UpdatePivotCache
  (bind _returnvalue (Transformation|GetActorLocation))
  (bind _outhit (Collision|LineTraceByChannel _returnvalue (+ _returnvalue (* (Math|Rotator|GetRotationXVector (Transformation|GetWorldRotation (Variables|Default|GetCamera))) (Variables|Default|GetMaxTraceDistance))) "TraceTypeQuery3" false 0 "None"))
  (Variables|Default|SetCachedRotationPivot (.Location (Collision|BreakHitResult _outhit)))
  (Variables|Default|SetbIsCachedPivotValid true))