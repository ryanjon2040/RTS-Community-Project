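; BP_Barrack is an RTS barracks structure that trains units and buys upgrades, triggered here by debug-style J and K key events.
; J buys the current upgrade, then switches the upgrade class to the second barracks tier.
; K spawns a civilian if game-state gold, wood and food cover a fixed cost, deducting it.
; Units spawn at a rotated offset, receive a controller and owner, then head to any rally point.
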(event `Key|J`
  (:`Pressed`
    (`self.BuyUpgrade` (`self.UpgradeClass`))
    (if true
      (set `self.UpgradeClass` "/Game/Blueprints/Upgrades/Structures/U_Barracks_2.U_Barracks_2_C"))))

(event `Key|K`
  (:`Pressed`
    (`self.SpawnUnit` "/Game/Blueprints/Characters/BP_Civilian.BP_Civilian_C")))

(event `SpawnUnit`
  (params (UnitClass :type "/Game/Blueprints/BP_RTS_Character Class Reference"))
  (bind _rallypoint (`self.RallyPoint`))
  (bind _asbp_rts_game_state (cast `/Game/Blueprints/BP_RTS_GameState` (`GameplayStatics.GetGameState`)))
  (bind (_resources_wood _resources_gold _resources_food) (break `/Game/Blueprints/BP_RTS_Resources` (`/Game/Blueprints/BP_RTS_GameState.Resources` _asbp_rts_game_state)))
  (if (and (>= _resources_gold 5) (>= _resources_wood 5) (>= _resources_food 5))
    (bind _asbp_rts_game_state_2 (cast `/Game/Blueprints/BP_RTS_GameState` (`GameplayStatics.GetGameState`)))
    (`/Game/Blueprints/BP_RTS_GameState.UpdateGold` _asbp_rts_game_state_2 -5)
    (`/Game/Blueprints/BP_RTS_GameState.UpdateWood` _asbp_rts_game_state_2 -5)
    (`/Game/Blueprints/BP_RTS_GameState.UpdateFood` _asbp_rts_game_state_2 -5)
    (bind _returnvalue (`|SpawnActorFromClass` UnitClass (`KismetMathLibrary.Conv_VectorToTransform` (+ (`self.K2_GetActorLocation`) (`KismetMathLibrary.GreaterGreater_VectorRotator` (`self.UnitSpawnLocation`) (`self.K2_GetActorRotation`)))) false true))
    (`Pawn.SpawnDefaultController` _returnvalue)
    (`/Game/Blueprints/BP_RTS_Character.SetPlayerState` _returnvalue (`self.OwnerPlayerState`))
    (if (!= _rallypoint null)
      (`/Game/Blueprints/BP_RTS_Character.Do_Action` _returnvalue (`SceneComponent.K2_GetComponentLocation` _rallypoint) null))))

(fn `UserConstructionScript`
  (`parent.UserConstructionScript`))